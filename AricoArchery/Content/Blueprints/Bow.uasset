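; Two-handed motion-controller bow: the first grab holds it, and a second grab pulls the string and spawns an arrow.
; While pulled, Tick aims the arrow through the holding hand's nock, feeds the grab point to the string material and drives haptics from draw changes.
; Releasing the string hand launches the arrow at a speed based on squared, clamped draw length.
; A spring-solve macro then eases the string back to rest.
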(event `self.ReceiveTick`
  (params (DeltaSeconds :type "Float (single-precision)"))
  (bind _returnvalue (`GameplayStatics.GetPlayerController` 0))
  (bind _stringmid (`self.StringMID`))
  (bind _returnvalue_2 (- (`SceneComponent.K2_GetComponentLocation` (select `/Game/Blueprints/Enum/LeftRight` (`self.HoldingHand`) :`NewEnumerator1` (`self.LeftSideNock`) :`NewEnumerator2` (`self.RightSideNock`))) (`self.CurGrabSpot`)))
  (`|ExecutionSequence`
    (:`then_1`
      ;[1 1 1] Pull String
      (if (`self.PullingString`)
        (bind _output_get (set `self.CurGrabSpot` (+ (`SceneComponent.K2_GetComponentLocation` (`Actor.RootComponent` (`self.StringHandBP`))) (`self.InitialStringGrabOffset`))))
        (`MaterialInstanceDynamic.SetScalarParameterValue` _stringmid "Grabbed" 1.0)
        (`MaterialInstanceDynamic.SetVectorParameterValue` _stringmid "GrabSpot" (`KismetMathLibrary.Conv_VectorToLinearColor` _output_get))
        (set `self.Length` (`KismetMathLibrary.VSize` (- (`SceneComponent.K2_GetComponentLocation` (`self.StringSphere`)) (`self.CurGrabSpot`))))
        (`self.K2_SetActorTransform` (`self.CurrentArrow`) (`KismetMathLibrary.MakeTransform` (+ (`self.CurGrabSpot`) (* (`KismetMathLibrary.Normal` _returnvalue_2) 30.0)) (`KismetMathLibrary.MakeRotFromX` _returnvalue_2)) false false)
        (`self.Haptics / Force Feedback`)
        (else
          ;[1 1 1] String Tension
          (bind _new_p (`self.Spring Solve` (`self.CurGrabSpot`) (`SceneComponent.K2_GetComponentLocation` (`self.String Mesh`)) 0.5 40.0 (`GameplayStatics.GetWorldDeltaSeconds`))
            (:`Out`
              (`MaterialInstanceDynamic.SetVectorParameterValue` (`self.StringMID`) "GrabSpot" (`KismetMathLibrary.Conv_VectorToLinearColor` _new_p))
              (set `self.CurGrabSpot` _new_p)
              (`PlayerController.SetHapticsByValue` _returnvalue 0.0 0.0 (select `/Game/Blueprints/Enum/LeftRight` (`self.StringPullHand`) :`NewEnumerator1` "Left" :`NewEnumerator2` "Right" :!type "EControllerHand Enum"))
              (`PlayerController.ClientPlayForceFeedback` _returnvalue null false false "None") ; Needs Force Feedback on Left and Right sides.
            )))))))

(fn `Grab Pressed`
  (params (`Which Hand` :type "/Game/Blueprints/Enum/LeftRight Enum" :default "NewEnumerator1") (`Hand BP` :type "/Game/Blueprints/Character/Hands/BP_LeftHand Object Reference"))
  (returns (`Grab Transform` :type "Transform Structure") (`Item Picked Up` :type Boolean) (`Secondary Grab` :type Boolean) (`Local Grab Location` :type "Vector Structure"))
  (locals (`Pick Up` :type Boolean))
  ;[1 1 1] Simple Grab
  (if (`self.Held`)
    ;[1 1 1] Grab String
    (set `self.StringPullHand` `Which Hand`)
    (set `self.StringHandBP` `Hand BP`)
    (set `self.PullingString` true)
    (set `local.Pick Up` false)
    (set `self.InitialStringGrabOffset` (- (`SceneComponent.K2_GetComponentLocation` (`self.StringSphere`)) (`SceneComponent.K2_GetComponentLocation` (`/Game/Blueprints/Character/Hands/BP_LeftHand.DefaultSceneRoot` (`self.StringHandBP`)))))
    (`SceneComponent.SetVisibility` (`self.String Release`) false false)
    ;[1 1 1] Spawn Arrow
    (bind _returnvalue (`|SpawnActorFromClass` "/Game/Blueprints/Arrow.Arrow_C" (`KismetMathLibrary.Conv_VectorToTransform` (0.0 0.0 0.0)) "AlwaysSpawn" "OverrideRootScale" null null))
    (set `self.CurrentArrow` _returnvalue)
    (else
      (set `self.HoldingHand` `Which Hand`)
      (set `self.Held` true)
      (set `self.PullingString` false)
      (set `local.Pick Up` true)))
  (return (`SceneComponent.K2_GetComponentToWorld` (`self.DefaultSceneRoot`)) (`local.Pick Up`) (`self.PullingString`) (`KismetMathLibrary.InverseTransformLocation` (`self.GetTransform`) (`SceneComponent.K2_GetComponentLocation` (`self.LeftSideNock`)))))

(fn `Grab Released`
  (params (`Which Hand` :type "/Game/Blueprints/Enum/LeftRight Enum" :default "NewEnumerator1"))
  (returns (`Drop On Release?` :type Boolean))
  (bind _projectilemovement (`/Game/Blueprints/Arrow.ProjectileMovement` (`self.CurrentArrow`)))
  (bind _returnvalue (* (`KismetMathLibrary.FClamp` (`self.Length`) 0.0 35.0) 2.0))
  (if (`|EnumEquality` `Which Hand` (`self.HoldingHand`))
    ;[1 1 1] Drop Weapon
    (set `self.Held` false)
    (set `self.PullingString` false)
    (set `self.Drop` true)
    (return (`self.Drop`))
    (else
      ;[1 1 1] Fire
      (`|ExecutionSequence`
        (:`then_0`
          (if (`self.PullingString`)
            (set `self.PullingString` false)
            (`ActorComponent.SetActive` _projectilemovement true false)
            (`ProjectileMovementComponent.SetVelocityInLocalSpace` _projectilemovement (`KismetMathLibrary.MakeVector` (* (* _returnvalue _returnvalue) 1.0)))
            (set `ProjectileMovementComponent.bRotationFollowsVelocity` true _projectilemovement)
            (set `self.CurrentArrow` null)
            (`PlayerController.ClientPlayForceFeedback` (`GameplayStatics.GetPlayerController` 0) null false false "None")))
        (:`then_1`
          (set `self.Drop` false)
          (return (`self.Drop`)))))))

(fn `Hand Begin Overlap`
  (params (`Which Hand` :type "/Game/Blueprints/Enum/LeftRight Enum" :default "NewEnumerator1") (`Hand BP` :type "/Game/Blueprints/Character/Hands/BP_LeftHand Object Reference"))
  (returns (Reply :type Boolean) (SelectionMID :type "MaterialInstanceDynamic Object Reference"))
  (if (`self.Held`)
    (if (not (`|EnumEquality` `Which Hand` (`self.HoldingHand`)))
      (`SceneComponent.SetVisibility` (`self.String Release`) true false)))
  (return true (select `bool` (`self.Held`) :`false` (select `/Game/Blueprints/Enum/LeftRight` `Which Hand` :`NewEnumerator1` (`self.LeftNockMID`) :`NewEnumerator2` (`self.RightNockMID`)) :`true` (`self.StringMID`))))

(fn `Hand End Overlap`
  (params (`Which Hand` :type "/Game/Blueprints/Enum/LeftRight Enum" :default "NewEnumerator1"))
  (returns (NewParam :type Boolean))
  (return false))

(fn `Haptics / Force Feedback`
  (bind _length (`self.Length`))
  (bind _returnvalue (- _length (`self.PrevLength`)))
  (bind _returnvalue_2 (`KismetMathLibrary.FClamp` (/ (`KismetMathLibrary.Abs` _returnvalue) 5.0)))
  (`PlayerController.SetHapticsByValue` (`GameplayStatics.GetPlayerController` 0) (`KismetMathLibrary.FClamp` (+ (/ _length 50.0) (/ _returnvalue 50.0))) _returnvalue_2 (select `/Game/Blueprints/Enum/LeftRight` (`self.StringPullHand`) :`NewEnumerator1` "Left" :`NewEnumerator2` "Right" :!type "EControllerHand Enum"))
  (if (> (`self.Time Accumulator`) 0.1)
    (`PlayerController.ClientPlayForceFeedback` (`GameplayStatics.GetPlayerController` 0) (`|GetArrayItem` (`self.RightForceFeedbacks`) (`KismetMathLibrary.FFloor` (* _returnvalue_2 10.0))) false false "None")
    (set `self.Time Accumulator` (+ (`self.Time Accumulator`) -0.1))
    (else
      (set `self.Time Accumulator` (+ (`self.Time Accumulator`) (`GameplayStatics.GetWorldDeltaSeconds`)))))
  (set `self.PrevLength` (`self.Length`))
  (return))

(fn `UserConstructionScript`)